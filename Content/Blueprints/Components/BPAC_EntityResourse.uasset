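; BPAC_EntityResourse is an actor component that stores a numeric resource value for an entity.
; InitializeResource sets the current value unless IsInitialized is true, though it never sets that flag itself.
; ModifyResource adds an amount, clamps the result between zero and MaxResource, and only prints a debug string on depletion.
; GetCurrentResource exposes the value, and the event graph holds no active logic.
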(fn `GetCurrentResource`
  (returns (ResourceValue :type "Float (double-precision)"))
  (return (`self.CurrentResource`)))

(fn `InitializeResource`
  (params (InitialValue :type "Float (double-precision)"))
  (locals (L_InitialValue :type "Float (double-precision)"))
  (set `local.L_InitialValue` InitialValue)
  (if (`self.IsInitialized`)
    (return)
    (else
      (set `self.CurrentResource` (`local.L_InitialValue`))
      (return))))

(fn `ModifyResource`
  (params (Amount :type "Float (double-precision)"))
  (locals (L_Amount :type "Float (double-precision)"))
  (set `local.L_Amount` Amount)
  (bind _output_get (set `self.CurrentResource` (`KismetMathLibrary.FClamp` (+ (`self.CurrentResource`) (`local.L_Amount`)) 0.0 (`self.MaxResource`))))
  (if (<= _output_get 0.0)
    (`KismetSystemLibrary.PrintString` "ResourceDepleted" true true (struct :`R` 0.771696 :`B` 1.0 :`A` 1.0) 5.0)
    (return)
    (else
      (return))))