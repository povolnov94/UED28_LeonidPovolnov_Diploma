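; BP_EnemyBase is the base enemy actor, delegating health, attack, death and AI management to components.
; On BeginPlay it binds damage handling and hooks its health bar widget to the HealthComponent.
; Damage reduces health, then either notifies BP_EnemyAIController of the player's attack or triggers the death action once, guarded by IsDead.
; Attacks go through the attack action component, and Tick draws the current patrol state as debug text.
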(event `self.ReceiveBeginPlay`
  (add `self.OnTakeAnyDamage` (`|CreateDelegate` :!event `ApplyDamage`))
  (bind _aswbp_enemy_health_bar (cast `/Game/HUD/WBP_EnemyHealthBar` (`WidgetComponent.GetUserWidgetObject` (`self.Widget`))))
  (`/Game/HUD/WBP_EnemyHealthBar.SetUpWidget` _aswbp_enemy_health_bar (`self.HealthComponent`)))

(event `self.ReceiveTick`
  (params (DeltaSeconds :type "Float (single-precision)"))
  (`KismetSystemLibrary.DrawDebugString` (+ (`SceneComponent.K2_GetComponentLocation` (`self.CapsuleComponent`)) (0.0 0.0 20.0)) (`KismetTextLibrary.Conv_TextToString` (`|FormatText` "{CurrentPatrolState} " (`|GetEnumeratorNameAsString` (`/Game/Components/BPAC_AIPatrolling.PatrolState` (`self.BPAC_AIManager`))))) null (struct :`G` 0.14996 :`B` 0.122139 :`A` 1.0)))

(fn `ApplyDamage`
  (params (DamagedActor :type "Actor Object Reference") (Damage :type "Float (single-precision)") (DamageType :type "DamageType Object Reference") (InstigatedBy :type "Controller Object Reference") (DamageCauser :type "Actor Object Reference"))
  (`/Game/Components/BPAC_EntityResourse.DecreaseValue` (`self.HealthComponent`) Damage)
  (if (> (`/Game/Components/BPAC_EntityResourse.GetCurValue` (`self.HealthComponent`)) 0.0)
    (bind _asbp_enemy_aicontroller (cast `/Game/Enemy/AI/BP_EnemyAIController` (`AIBlueprintHelperLibrary.GetAIController` self)))
    (`/Game/Enemy/AI/BP_EnemyAIController.Attacked by Player` _asbp_enemy_aicontroller)
    (else
      (`self.StartDeath`))))

(fn `AttackPlayer`
  (params (AttackingActor :type "Actor Object Reference"))
  (`/Game/Components/BPAC_ActionBase.StartAction` :`self` (`self.BPAC_AttackAction`) :`TargetActor` AttackingActor))

(fn `InteractionInterface`
  (params (Interactor :type "Actor Object Reference"))
  (returns (Success :type Boolean))
  (return true))

(fn `StartDeath`
  (if (not (`self.IsDead`))
    (`/Game/Components/BPAC_ActionBase.StartAction` :`self` (`self.BPAC_DeathAction`))
    (set `self.IsDead` true)))

(fn `UserConstructionScript`)