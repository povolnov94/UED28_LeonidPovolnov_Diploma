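; Interactive door Blueprint that players can open, close or unlock through an interaction interface.
; A box collision adds the door to an overlapping actor's interaction queue and removes it when the overlap ends.
; Interacting switches on the door's current state: opened doors close, closed doors open, locked doors only unlock, and doors mid-action ignore the request.
; Construction defers to the parent class.
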(event `self.BoxCollision.OnComponentBeginOverlap`
  (params (OverlappedComponent :type "PrimitiveComponent Object Reference") (OtherActor :type "Actor Object Reference") (OtherComp :type "PrimitiveComponent Object Reference") (OtherBodyIndex :type Integer) (bFromSweep :type Boolean) (SweepResult :type "HitResult Structure (by ref)"))
  (`/Game/Components/BPFL_Utility.AddToInteractionQueue` self OtherActor))

(event `self.BoxCollision.OnComponentEndOverlap`
  (params (OverlappedComponent :type "PrimitiveComponent Object Reference") (OtherActor :type "Actor Object Reference") (OtherComp :type "PrimitiveComponent Object Reference") (OtherBodyIndex :type Integer))
  (`/Game/Components/BPFL_Utility.RemoveFromInteractionQueue` self OtherActor))

(fn `InteractionInterface`
  (returns (Success :type Boolean))
  (switch `/Game/Enviroment/Doors/ENUM_DoorState` (`self.GetCurrentState`)
    (:`NewEnumerator0`
      (bind _success (`self.Close`))
      (return _success))
    (:`NewEnumerator1`
      (bind _success_2 (`self.Open`))
      (return _success_2))
    (:`NewEnumerator2`
      (bind _success_3 (`self.SetIsLocked` null))
      (return _success_3))
    (:`NewEnumerator3`
      (return false))))

(fn `UserConstructionScript`
  (`parent.UserConstructionScript`))