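; BP_Base_Target is a base target actor that can be damaged and destroyed.
; It forwards AnyDamage to TakeDamage, which lowers its BPACHealth component and destroys the actor once health reaches zero or below.
; Every tick it prints its name with current and max HP on screen as a debug readout.
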(event `self.ReceiveTick`
  (params (DeltaSeconds :type "Float (single-precision)"))
  (bind _bpac_health (`self.BPAC_Health`))
  (`KismetSystemLibrary.PrintString` (`KismetTextLibrary.Conv_TextToString` (`|FormatText` "{Name} HP : {Current} / {Max}" self (`/Game/Components/BPAC_EntityResourse.GetCurValue` _bpac_health) (`/Game/Components/BPAC_EntityResourse.MaxValue` _bpac_health))) true false (struct :`R` 1.0 :`G` 0.717968 :`A` 1.0) 0.0))

(event `self.ReceiveAnyDamage`
  (params (Damage :type "Float (single-precision)") (DamageType :type "DamageType Object Reference") (InstigatedBy :type "Controller Object Reference") (DamageCauser :type "Actor Object Reference"))
  (`self.TakeDamage` Damage))

(fn `TakeDamage`
  (params (Amount :type "Float (double-precision)"))
  (`/Game/Components/BPAC_EntityResourse.DecreaseValue` (`self.BPAC_Health`) Amount)
  (if (<= (`/Game/Components/BPAC_EntityResourse.GetCurValue` (`self.BPAC_Health`)) 0.0)
    (`self.K2_DestroyActor`)
    (return)
    (else
      (return))))

(fn `UserConstructionScript`)