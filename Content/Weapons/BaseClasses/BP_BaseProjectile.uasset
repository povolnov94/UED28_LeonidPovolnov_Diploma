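; BP_BaseProjectile is a base weapon projectile that flies along a set direction and damages what it hits.
; On BeginPlay it sets the ProjectileMovement velocity from the component's initial speed and its Direction variable.
; On Hit it applies its Damage and DamageType to the other actor, naming itself as damage causer, then destroys itself.
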(event `self.ReceiveBeginPlay`
  (set `MovementComponent.Velocity` (* (`ProjectileMovementComponent.InitialSpeed` (`self.ProjectileMovement`)) (`self.Direction`)) (`self.ProjectileMovement`)))

(event `self.ReceiveHit`
  (params (MyComp :type "PrimitiveComponent Object Reference") (Other :type "Actor Object Reference") (OtherComp :type "PrimitiveComponent Object Reference") (bSelfMoved :type Boolean) (HitLocation :type "Vector Structure") (HitNormal :type "Vector Structure") (NormalImpulse :type "Vector Structure") (Hit :type "HitResult Structure (by ref)"))
  (`GameplayStatics.ApplyDamage` Other (`KismetMathLibrary.Conv_IntToDouble` (`self.Damage`)) null self "/Script/Engine.DamageType")
  (`self.K2_DestroyActor`))

(fn `UserConstructionScript`)