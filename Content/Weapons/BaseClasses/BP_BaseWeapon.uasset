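; BP_BaseWeapon is a base weapon actor that handles firing, ammo and reloading, driven by a WeaponData configuration.
; StartShooting runs a looping rate-of-fire timer, and StopShooting sets a one-shot timer for the remaining interval.
; MakeShot traces from the owner's camera or eyes, calls OnMakeShot, then spawns an aimed projectile or applies hitscan damage.
; Reloading refills from reserve ammo and updates the owner's BPAC_WeaponManeger state, while Tick prints debug ammo.
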(event `self.ReceiveBeginPlay`
  (set `self.OwnerCamera` (`self.GetComponentByClass` (`self.GetOwner`) "/Script/Engine.CameraComponent"))
  (`SceneComponent.K2_AttachToComponent` (`self.MuzzleFX`) (`self.WeaponMesh`) (`self.MuzzleFXSocketName`) "KeepRelative" "KeepRelative" "KeepRelative" true)
  (set `self.CurrentAmmo` (`.AmmoCapacity_34_D26683344976E62E791BD79DC3121DA1` (break `/Game/Weapons/S_WeaponData` (`self.WeaponData`))))
  (set `self.TotalAmmo` (`.TotalAmmo_36_E908045B4C2806571BA0E3B0ECB1EF0A` (break `/Game/Weapons/S_WeaponData` (`self.WeaponData`)))))

(event `OnMakeShot`
  (params (Hit :type "HitResult Structure")))

(event `self.ReceiveTick`
  (params (DeltaSeconds :type "Float (single-precision)"))
  (`KismetSystemLibrary.PrintString` (`KismetTextLibrary.Conv_TextToString` (`|FormatText` "{WeaponName} - Ammo {Current} / {Max}" (`KismetStringLibrary.Conv_IntToString` (`self.CurrentAmmo`)) (`KismetStringLibrary.Conv_IntToString` (`self.TotalAmmo`)) self)) true true (struct :`G` 0.208333 :`B` 0.044066 :`A` 1.0) 0.0))

(fn `IsEnableForShooting`
  (set `self.IsReadyForShoot` true)
  (return))

(fn `IsFullAmmo`
  (returns (Success :type Boolean))
  (return (!= (`self.CurrentAmmo`) (`.AmmoCapacity_34_D26683344976E62E791BD79DC3121DA1` (break `/Game/Weapons/S_WeaponData` (`self.WeaponData`))))))

(fn `MakeShot`
  (bind (_ammotype _damage _rateoffire _reloadtime _projectileclass) (break `/Game/Weapons/S_WeaponData` (`self.WeaponData`)))
  (bind (_outlocation _outrotation) (`self.GetActorEyesViewPoint` (`self.GetOwner`)))
  (if (> (`self.CurrentAmmo`) 0)
    (`/Engine/EditorBlueprintResources/StandardMacros.IsValid` (`self.OwnerCamera`)
      (:`Is Valid`
        (bind _desiredview (`CameraComponent.GetCameraView` (`self.OwnerCamera`) 0.0))
        (bind (_location _rotation) (break `MinimalViewInfo` _desiredview))
        (set `self.StartPoint` _location)
        (set `self.EndPoint` (+ (`self.StartPoint`) (* (`KismetMathLibrary.Conv_RotatorToVector` _rotation) (`self.TraceLengh`)))))
      (:`Is Not Valid`
        (set `self.StartPoint` _outlocation)
        (set `self.EndPoint` (+ (`self.StartPoint`) (* (`KismetMathLibrary.Conv_RotatorToVector` _outrotation) (`self.TraceLengh`))))))
    (bind (_outhit _returnvalue) (`KismetSystemLibrary.LineTraceSingle` (`self.StartPoint`) (`self.EndPoint`) "TraceTypeQuery2" false (`|MakeArray` (`self.GetOwner`)) "ForDuration" false (struct :`R` 1.0 :`A` 1.0) (struct :`G` 1.0 :`A` 1.0) 2.0))
    (`self.OnMakeShot` _outhit)
    (set `self.CurrentAmmo` (- (`self.CurrentAmmo`) 1))
    (switch `/Game/Weapons/ENUM_AmmoType` (`.AmmoType_8_237F03B8426266CD473BB6B07E377543` (break `/Game/Weapons/S_WeaponData` (`self.WeaponData`)))
      (:`NewEnumerator0`
        (bind (_bblockinghit _binitialoverlap _time _distance _location_2 _impactpoint _normal _impactnormal _physmat _hitactor _hitcomponent _hitbonename _bonename _hititem _elementindex _faceindex _tracestart _traceend) (`GameplayStatics.BreakHitResult` _outhit))
        (`|SpawnActorFromClass` _projectileclass (`KismetMathLibrary.MakeTransform` (`SceneComponent.GetSocketLocation` (`self.WeaponMesh`) (`self.MuzzleFXSocketName`))) "AdjustIfPossibleButAlwaysSpawn" "MultiplyWithRoot" (`self.GetOwner`) (`KismetMathLibrary.Normal` (- (`KismetMathLibrary.SelectVector` _impactpoint _traceend _returnvalue) (`SceneComponent.GetSocketLocation` (`self.WeaponMesh`) (`self.MuzzleFXSocketName`)))) _damage null)
        (return))
      (:`NewEnumerator1`
        (`GameplayStatics.ApplyDamage` _hitactor (`KismetMathLibrary.Conv_IntToDouble` (`.Damage_5_05EDF7CC4C05AB4F4355A5B90A99FD9C` (break `/Game/Weapons/S_WeaponData` (`self.WeaponData`)))) (`self.OwnerController`) self)
        (return)))))

(fn `Reloading`
  (set `self.AmmoNeeded` (- (`.AmmoCapacity_34_D26683344976E62E791BD79DC3121DA1` (break `/Game/Weapons/S_WeaponData` (`self.WeaponData`))) (`self.CurrentAmmo`)))
  (if (>= (`self.TotalAmmo`) (`self.AmmoNeeded`))
    (set `self.CurrentAmmo` (+ (`self.AmmoNeeded`) (`self.CurrentAmmo`)))
    (set `self.TotalAmmo` (- (`self.TotalAmmo`) (`self.AmmoNeeded`)))
    (set `/Game/Components/BPAC_WeaponManeger.CurrentState` "NewEnumerator2" (`self.GetComponentByClass` (`self.GetOwner`) "/Game/Components/BPAC_WeaponManeger.BPAC_WeaponManeger_C"))
    (return)
    (else
      (set `self.CurrentAmmo` (+ (`self.CurrentAmmo`) (`self.TotalAmmo`)))
      (set `self.TotalAmmo` 0)
      (set `/Game/Components/BPAC_WeaponManeger.CurrentState` "NewEnumerator2" (`self.GetComponentByClass` (`self.GetOwner`) "/Game/Components/BPAC_WeaponManeger.BPAC_WeaponManeger_C"))
      (return))))

(fn `Start Reloading`
  (`KismetSystemLibrary.K2_SetTimerDelegate` (`|CreateDelegate` :!event `Reloading`) (`.ReloadTime_15_8B0300584C386225C2D8B28061AC3C8E` (break `/Game/Weapons/S_WeaponData` (`self.WeaponData`))))
  (return))

(fn `StartShooting`
  (returns (Success :type Boolean))
  (if (`self.IsReadyForShoot`)
    (bind _aspawn (cast `Pawn` (`self.GetOwner`)))
    (set `self.OwnerController` (`Pawn.GetController` _aspawn))
    (`self.MakeShot`)
    (`self.StartShootTimer` (`|CreateDelegate` :!event `MakeShot`))
    (set `self.IsReadyForShoot` false)
    (return true)
    (else
      (return false))))

(fn `StartShootTimer`
  (params (Event :type Delegate))
  (bind _returnvalue (`KismetSystemLibrary.K2_SetTimerDelegate` Event (`.RateOfFire_13_6B1304034A722065FD20F395708FA3D7` (break `/Game/Weapons/S_WeaponData` (`self.WeaponData`))) true))
  (set `self.ShootTimer` _returnvalue))

(fn `StopShooting`
  (returns (Success :type Boolean))
  (if (`KismetSystemLibrary.K2_IsTimerActiveHandle` (`self.ShootTimer`))
    (`KismetSystemLibrary.K2_SetTimerDelegate` (`|CreateDelegate` :!event `IsEnableForShooting`) (`KismetSystemLibrary.K2_GetTimerRemainingTimeHandle` (`self.ShootTimer`)))
    (`KismetSystemLibrary.K2_ClearAndInvalidateTimerHandle` (`self.ShootTimer`))
    (return true)
    (else
      (return false))))

(fn `UserConstructionScript`)