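; BP_Pickup_BaseWeapon is a base pickup that gives a weapon to the actor it is activated on.
; ActivatePickupEffect finds the target's BPAC_WeaponManeger component, passes WeaponClass to its AddWeapon and returns that result, or false when the component is missing.
; Overlap and construction logic only forward to the parent class.
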(event `self.ReceiveActorBeginOverlap`
  (params (OtherActor :type "Actor Object Reference"))
  (`parent.ReceiveActorBeginOverlap` OtherActor))

(fn `ActivatePickupEffect`
  (params (TargetActor :type "Actor Object Reference"))
  (returns (Success :type Boolean))
  (locals (L_WeaponManager :type "/Game/Components/BPAC_WeaponManeger Object Reference"))
  (bind _output_get (set `local.L_WeaponManager` (`self.GetComponentByClass` TargetActor "/Game/Components/BPAC_WeaponManeger.BPAC_WeaponManeger_C")))
  (`/Engine/EditorBlueprintResources/StandardMacros.IsValid` _output_get
    (:`Is Valid`
      (bind _success (`/Game/Components/BPAC_WeaponManeger.AddWeapon` (`local.L_WeaponManager`) (`self.WeaponClass`)))
      (return _success))
    (:`Is Not Valid`
      (return false))))

(fn `UserConstructionScript`
  (`parent.UserConstructionScript`))